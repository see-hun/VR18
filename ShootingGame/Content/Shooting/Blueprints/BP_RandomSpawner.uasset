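; BP_RandomSpawner spawns a randomly chosen actor from its Actors list at its own transform.
; On BeginPlay, only the authority runs the first spawn, and each spawned actor's OnDestroyed event is bound.
; EventItemDestroy sets a fixed-delay timer that calls DoSpawnItem again by function name, so a new random item replaces the destroyed one.
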(event EventBeginPlay
  (Networking|SwitchHasAuthority
    (:Authority
      (CallFunction|DoSpawnItem))))

(fn ConstructionScript)

(fn EventItemDestroy
  (params (DestroyedActor :type Actor%20Object%20Reference))
  (Utilities|Time|SetTimerbyFunctionName 0 "DoSpawnItem" 2e+01))

(fn DoSpawnItem
  (bind _returnvalue (Game|SpawnActorfromClass (.OutItem (Utilities|Array|Random (Variables|Default|GetActors))) (Transformation|GetActorTransform) "Undefined" "MultiplyWithRoot" 0 0))
  (Game|BindEventtoOnDestroyed _returnvalue (EventDispatchers|CreateEvent :!event EventItemDestroy)))