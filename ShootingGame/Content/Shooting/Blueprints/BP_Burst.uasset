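; BP_Burst is a burst-fire weapon Blueprint that fires up to three shots per trigger press.
; EventTrigger resets the shot count, fires at once, then starts a looping SingleShoot timer at the WeaponData fire rate.
; SingleShoot plays the rifle fire montage on the owning character and clears the timer after the third shot or when IsCanShoot fails.
; Releasing the trigger does not interrupt the burst.
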(event EventBeginPlay)

(event Collision|EventActorBeginOverlap
  (params (OtherActor :type Actor%20Object%20Reference)))

(event EventTick
  (params (DeltaSeconds :type Float%20%28single-precision%29)))

(fn ConstructionScript
  (|CallParentFunction))

(fn SingleShoot
  (if (CallFunction|IsCanShoot)
    (bind _ownchar (Variables|Default|GetOwnChar) ; OwnChar 변수가 \n정상적인 값이라면 개속 실행
      (:then
        (Animation|PlayAnimMontage _ownchar "/Game/Characters/Mannequins/Animations/Rifle/MM_Rifle_Fire_Montage.MM_Rifle_Fire_Montage" 1.0 "None") ; Target에 연결되어 있는 OwnChar에 Montage 에니메이션 실행\nAnim Montage는 MM_Rifle_Fire
        (bind _output_get (Variables|Default|SetShootCnt (+ (Variables|Default|GetShootCnt) 1)))
        (if (>= _output_get 3)
          (Utilities|Time|ClearTimerbyFunctionName 0 "SingleShoot")))
      (:else))
    (else
      (Utilities|Time|ClearTimerbyFunctionName 0 "SingleShoot"))))

(fn EventTrigger
  (params (IsPress :type Boolean))
  (if IsPress
    (Variables|Default|SetShootCnt 0)
    (CallFunction|SingleShoot)
    (Utilities|Time|SetTimerbyFunctionName 0 "SingleShoot" (.firerate (Variables|Default|GetWeaponData)) true)
    (return false)))