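; Replicated, data-driven weapon actor that attaches to a character's weapon socket and handles firing, reloading and dropping with physics.
; Trigger and reload events play rifle montages; separate notify events spawn muzzle effects and, for the local player only, send server requests.
; The server consumes ammo, line-traces from the camera aim to apply damage, and refills from PlayerState magazines.
; Ammo's RepNotify updates the local HUD.
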(event Custom|ReqFire
  (params (FireLocation :type Vector) (FireForwardVector :type Vector))
  ;[1 0 0] (Server)
  (bind _isused (CallFunction|UseAmmo))
  (if _isused
    (bind _outhit (Collision|LineTraceForObjects FireLocation (+ FireLocation (* FireForwardVector 5e+03)) (Utilities|Array|MakeArray "ObjectTypeQuery1" "ObjectTypeQuery2" "ObjectTypeQuery3" "ObjectTypeQuery4" "ObjectTypeQuery6") false 0 "None" true "(R=1.000000,G=0.000000,B=0.000000,A=1.000000)" "(R=0.000000,G=1.000000,B=0.000000,A=1.000000)" 2e+01))
    ;[1 1 1] Damaged Actor : 맞은 사람
    ; Event Instigator : 때린 사람
    ; Damage Causer : 칼, 총, 도끼, 망치, 수류탄
    (Game|Damage|ApplyDamage (.HitActor (Collision|BreakHitResult _outhit)) (.damage (Variables|Default|GetWeaponData)) (Pawn|GetController (Variables|Default|GetOwnChar)) self)))

(event Custom|ReqReload
  ;[1 0 0] (Server)
  (bind _asbp_shooting_player_state (Utilities|Casting|CastToBP_ShootingPlayerState (Variables|/Script/Engine.Pawn|GetPlayerState (Variables|Default|GetOwnChar))))
  (bind _isused (Default|UseMag _asbp_shooting_player_state))
  (if _isused
    (Variables|Default|SetAmmo (.maxammo (Variables|Default|GetWeaponData))) ; 30으로 Ammo 변수 값을 변경하고\n변경 Event를 OnRep_Ammo 함수로 Client에 알려준다
  ))

(event EventBeginPlay
  (Components|StaticMesh|SetStaticMesh (Variables|Default|GetStaticMesh) (.staticmesh (Variables|Default|GetWeaponData))))

(fn ConstructionScript)

(fn DoEquipWeapon
  (params (Character :type Character%20Object%20Reference))
  (bind _staticmesh (Variables|Default|GetStaticMesh))
  ;[1 1 1] Own Char에 Character 값을 저장한다
  (Variables|Default|SetOwnChar Character)
  (Variables|/Script/Engine.Pawn|SetbUseControllerRotationYaw Character true) ; Target에 연결되어있는 Character에 Use Controller Rotation Yaw 값을 True 설정해서\nControl(즉 플레이어) 카메라 방향을 따라서 캐릭터가 회전하도록 한다
  (Physics|SetSimulatePhysics _staticmesh false) ; Target에 연결되어 있는 Static Mesh에 물리적인 시뮬레이션을 비활성화 한다
  (Collision|SetCollisionEnabled _staticmesh "NoCollision") ; Target에 연결되어 있는 Static Mesh에 Collision을\nQuery(이벤트)와 Physics(물리)를 전부 비활성화 한다
  (Transformation|AttachComponentToComponent _staticmesh (Variables|/Script/Engine.Character|GetMesh Character) "weapon" "SnapToTarget" "SnapToTarget" "SnapToTarget" true) ; Target에 연결되어 있는 StaticMesh를 Parent에 열결 되어있는\nCharacter - Mesh에 붙인다\nMesh에 weapon 이름에 Socket Name이 있다면 Snap to Target( Socket에 붙는다) 한다
  (CallFunction|UpdateUIAmmo) ; Update UIAmmo 함수를 호출한다
)

(fn DoUnEquipWeapon
  (params (Character :type Character%20Object%20Reference))
  (bind _staticmesh (Variables|Default|GetStaticMesh))
  (Variables|/Script/Engine.Pawn|SetbUseControllerRotationYaw Character false) ; Target에 연결되어있는 Character에 Use Controller Rotation Yaw 값을 False 설정해서\nControl(즉 플레이어) 카메라 방향을 따라서 캐릭터가 회전하지 않도록 한다
  (Collision|SetCollisionEnabled _staticmesh "QueryAndPhysics") ; Target에 연결되어 있는 Static Mesh에 Collision을\nQuery(이벤트)와 Physics(물리)를 전부 활성화 한다
  (Physics|SetSimulatePhysics _staticmesh true) ; Target에 연결되어 있는 Static Mesh에 물리적인 시뮬레이션을 활성화 한다
  (Transformation|DetachFromComponent _staticmesh "KeepWorld" "KeepWorld" "KeepWorld" true) ; Target에 연결되어있는  StaticMesh에 모든 것을 Detach(때어내다)한다\n때어 낼때 Location, Rotation, Scale을 Keep World(월드 위치 기준으로 한다)로 한다.
)

(fn NotifyFire
  (bind _returnvalue (Game|GetPlayerCameraManager 0))
  (bind _staticmesh (Variables|Default|GetStaticMesh))
  (bind _returnvalue_2 (Transformation|GetActorLocation _returnvalue))
  (bind _returnvalue_3 (Transformation|GetSocketTransform _staticmesh "muzzle" "RTS_World"))
  (bind _returnvalue_4 (Transformation|GetActorForwardVector _returnvalue))
  ;[1 1 1] 모든 클라이언트가 전부 실행해야 되는 곳
  (Effects|SpawnEmitteratLocation (.effect (Variables|Default|GetWeaponData)) (.location _returnvalue_3) (.rotation _returnvalue_3) "0.100000,0.100000,0.100000")
  (Audio|SpawnSoundatLocation (.sound (Variables|Default|GetWeaponData)) (.location _returnvalue_3) "0, 0, 0" 1.0 1.0 0.0 0 0)
  ;[1 1 1] OwnChar와 PlayerCharacter 0번(즉 컨트롤하고 있는 Character)과 비교해서 같으면 개속 실행
  (if (== (Variables|Default|GetOwnChar) (Game|GetPlayerCharacter 0))
    ;[1 1 1] 소유한 클라이언트만 실행해야되는 곳
    (CallFunction|ReqFire (+ _returnvalue_2 (* _returnvalue_4 (Math|Vector|Distance(Vector) _returnvalue_2 (.location _returnvalue_3)))) _returnvalue_4) ; 서버에 ReqFire 함수 호출
  ))

(fn UpdateUIAmmo
  ;[1 1 1] OwnChar와 PlayerCharacter 0번(즉 컨트롤하고 있는 Character)과 비교해서 같으면 개속 실행
  (if (== (Variables|Default|GetOwnChar) (Game|GetPlayerCharacter 0))
    ;[1 1 1] Player Controller 0번에 HUD를 BP_ShootingHud로 호출해서 정상적이라면 다음 실행
    (bind _asbp_shooting_hud (Utilities|Casting|CastToBP_ShootingHud (HUD|GetHUD (Game|GetPlayerController 0))))
    (Default|UpdateAmmo _asbp_shooting_hud (Variables|Default|GetAmmo)) ; Target에 연결되어있는 BP_Shooting Hud에 Update Ammo 함수를\nAmmo 변수에 BP_Weapon에 Ammo 변수 값을 전달하여 호출
  ))

(fn OnRepAmmo
  (CallFunction|UpdateUIAmmo) ; Update UIAmmo 함수를 호출한다
)

(fn UseAmmo
  (if (> (Variables|Default|GetAmmo) 0)
    (Variables|Default|SetAmmo (Math|Integer|Clamp(Integer) (- (Variables|Default|GetAmmo) 1) 0 (.maxammo (Variables|Default|GetWeaponData)))) ; Ammo에 연결된 값으로 Ammo 변수 값을 변경하고\n변경 Event를 OnRep_Ammo 함수로 Client에 알려준다
    (return true)
    (else
      (return false))))

(fn IsCanReload
  (bind _asbp_shooting_player_state (Utilities|Casting|CastToBP_ShootingPlayerState (Variables|/Script/Engine.Pawn|GetPlayerState (Variables|Default|GetOwnChar)))
    (:then
      (return (Default|IsCanReload _asbp_shooting_player_state)))
    (:CastFailed
      (return false))))

(fn IsCanShoot
  (return (> (Variables|Default|GetAmmo) 0)))

(fn EventEquipWeapon
  (params (Character :type Character%20Object%20Reference))
  ;[1 1 1] Do Equip Weapon 함수를 Character 변수 값을 전달하여 호출한다
  (CallFunction|DoEquipWeapon Character)
  (return true))

(fn EventNotifyFire
  (CallFunction|NotifyFire) ; Notify Fire 함수 실행
  (return true))

(fn EventNotifyReload
  ;[1 1 1] OwnChar와 PlayerCharacter 0번(즉 컨트롤하고 있는 Character)과 비교해서 같으면 개속 실행
  (if (== (Variables|Default|GetOwnChar) (Game|GetPlayerCharacter 0))
    (CallFunction|ReqReload) ; 서버에 ReqReload 함수 호출
    (return true)))

(fn EventReload
  (if (CallFunction|IsCanReload)
    (bind _ownchar (Variables|Default|GetOwnChar) ; OwnChar 변수가 \n정상적인 값이라면 개속 실행
      (:then
        (Animation|PlayAnimMontage _ownchar "/Game/Characters/Mannequins/Animations/Rifle/MM_Rifle_Reload_Montage.MM_Rifle_Reload_Montage" 1.0 "None") ; Target에 연결되어 있는 OwnChar에 Montage 에니메이션 실행\nAnim Montage는 MM_Rifle_Reload
        (return true))
      (:else))))

(fn EventTrigger
  (params (IsPress :type Boolean))
  (if IsPress
    (if (CallFunction|IsCanShoot)
      (bind _ownchar (Variables|Default|GetOwnChar) ; OwnChar 변수가 \n정상적인 값이라면 개속 실행
        (:then
          (Animation|PlayAnimMontage _ownchar "/Game/Characters/Mannequins/Animations/Rifle/MM_Rifle_Fire_Montage.MM_Rifle_Fire_Montage" 1.0 "None") ; Target에 연결되어 있는 OwnChar에 Montage 에니메이션 실행\nAnim Montage는 MM_Rifle_Fire
          (return true))
        (:else)))))

(fn EventUnEquipWeapon
  (params (Character :type Character%20Object%20Reference))
  ;[1 1 1] Do Un Equip Weapon 함수를 Character 변수에 Character 변수에 값을 전달해서 호출한다
  (CallFunction|DoUnEquipWeapon Character)
  (return true))