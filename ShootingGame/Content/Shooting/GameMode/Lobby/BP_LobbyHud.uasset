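; BP_LobbyHud is the lobby HUD that shows the player list.
; On BeginPlay it creates a LobbyHudWidget, adds it to the viewport and refreshes its player list.
; BindPlayerState subscribes to a player state's user-name change dispatcher and immediately runs EventChangeUserName with the current name.
; That handler refreshes the list if the widget is valid, with debug prints tracing both functions.
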(event EventBeginPlay
  (bind _returnvalue (UserInterface|CreateWidget "/Game/Shooting/Widget/Lobby/LobbyHudWidget.LobbyHudWidget_C"))
  (bind _output_get (Variables|Default|SetHudWidget _returnvalue))
  (UserInterface|Viewport|AddtoViewport _output_get 0)
  (Default|UpdatePlayerList (Variables|Default|GetHudWidget)))

(fn ConstructionScript)

(fn BindPlayerState
  (params (PlayerState :type BP%20Lobby%20Player%20State%20Object%20Reference))
  (Development|PrintString "BindPlayerState" true true "(R=0.000000,G=0.660000,B=1.000000,A=1.000000)" 6e+01)
  (EventDispatchers|BindEventtoEventDispatcherChangeUserName PlayerState (EventDispatchers|CreateEvent :!event EventChangeUserName))
  (CallFunction|EventChangeUserName (Variables|/Game/Shooting/GameMode/Lobby/BP_LobbyPlayerState.BP_LobbyPlayerState_C|GetUserName PlayerState)))

(fn EventChangeUserName
  (params (UserName :type String))
  (bind _hudwidget (Variables|Default|GetHudWidget))
  (Development|PrintString (Utilities|String|Append "Event Change User Name - " UserName) true true "(R=0.000000,G=0.660000,B=1.000000,A=1.000000)" 6e+01)
  (Utilities|IsValid _hudwidget
    (:Is%20Valid
      (Default|UpdatePlayerList _hudwidget))))