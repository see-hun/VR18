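; Lobby player state that holds a replicated user name and announces changes to it.
; On BeginPlay it gets the HUD of player controller 0 and, if that is a BP_LobbyHud, binds itself to it.
; ChangeUserName sets the name, and its RepNotify prints a debug message and fires the ChangeUserName event dispatcher with the new value.
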(event EventBeginPlay
  (bind _asbp_lobby_hud (Utilities|Casting|CastToBP_LobbyHud (HUD|GetHUD (Game|GetPlayerController 0))))
  (Default|BindPlayerState _asbp_lobby_hud self))

(fn ConstructionScript)

(fn ChangeUserName
  (params (NewUserName :type String))
  (Variables|Default|SetUserName NewUserName))

(fn OnRepUserName
  (Development|PrintString (Utilities|String|Append "On Rep User Name - " (Variables|Default|GetUserName)) true true "(R=0.000000,G=0.660000,B=1.000000,A=1.000000)" 6e+01)
  (Default|CallEventDispatcherChangeUserName (Variables|Default|GetUserName)))