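; BP_ShootingHud is the shooting game's in-game HUD, which creates ShootingHudWidget on BeginPlay and switches to game-only input with the cursor hidden.
; It binds to the local BP_ShootingPlayerState's HP, magazine and SH dispatchers and pushes initial values to the widget, retrying on a short timer until the state exists.
; BindPlayerState hooks a given player's name and kill/death changes to refresh the widget's player list.
; UpdateAmmo forwards ammo to the widget.
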(event EventBeginPlay
  (bind _returnvalue (Game|GetPlayerController 0))
  (Development|PrintString "Hud" true true "(R=0.000000,G=0.660000,B=1.000000,A=1.000000)" 6e+01)
  (bind _returnvalue_2 (UserInterface|CreateWidget "/Game/Shooting/Widget/InGame/ShootingHudWidget.ShootingHudWidget_C"))
  (bind _output_get (Variables|Default|SetHudWidget _returnvalue_2))
  (UserInterface|Viewport|AddtoViewport _output_get 0)
  (CallFunction|BindMyPlayerState)
  (Input|SetInputModeGameOnly _returnvalue false)
  (Variables|/Script/Engine.PlayerController|SetbShowMouseCursor _returnvalue false))

(fn ConstructionScript)

(fn UpdateAmmo
  (params (Ammo :type Integer))
  (Default|UpdateAmmo (Variables|Default|GetHudWidget) Ammo) ; Target에 연결되어있는 HudWidget에 Update Ammo 함수를 Ammo값을 전달하여 호출
)

(fn UpdateHp
  (params (CurHp :type Float%20%28double-precision%29) (MaxHp :type Float%20%28double-precision%29))
  (Default|UpdateHp (Variables|Default|GetHudWidget) CurHp MaxHp))

(fn BindMyPlayerState
  (bind _asbp_shooting_player_state (Utilities|Casting|CastToBP_ShootingPlayerState (Variables|/Script/Engine.Controller|GetPlayerState (Game|GetPlayerController 0)))
    (:then
      (EventDispatchers|BindEventtoEventDispatcherUpdateHp _asbp_shooting_player_state (EventDispatchers|CreateEvent :!event UpdateHp))
      (CallFunction|UpdateHp (Variables|/Game/Shooting/GameMode/InGame/BP_ShootingPlayerState.BP_ShootingPlayerState_C|GetCurHp _asbp_shooting_player_state) (Variables|/Game/Shooting/GameMode/InGame/BP_ShootingPlayerState.BP_ShootingPlayerState_C|GetMaxHp _asbp_shooting_player_state))
      (EventDispatchers|BindEventtoEventDispatcherUpdateMag _asbp_shooting_player_state (EventDispatchers|CreateEvent :!event UpdateMag))
      (CallFunction|UpdateMag (Variables|/Game/Shooting/GameMode/InGame/BP_ShootingPlayerState.BP_ShootingPlayerState_C|GetMag _asbp_shooting_player_state))
      (EventDispatchers|BindEventtoEventDispatcherUpdateSH _asbp_shooting_player_state (EventDispatchers|CreateEvent :!event UpdateSH))
      (CallFunction|UpdateSH (Variables|/Game/Shooting/GameMode/InGame/BP_ShootingPlayerState.BP_ShootingPlayerState_C|GetCurSH _asbp_shooting_player_state) (Variables|/Game/Shooting/GameMode/InGame/BP_ShootingPlayerState.BP_ShootingPlayerState_C|GetMaxSH _asbp_shooting_player_state)))
    (:CastFailed
      (Utilities|Time|SetTimerbyFunctionName 0 "BindMyPlayerState" 0.01))))

(fn UpdateMag
  (params (Mag :type Integer))
  (Default|UpdateMag (Variables|Default|GetHudWidget) Mag))

(fn UpdateSH
  (params (CurSH :type Float%20%28double-precision%29) (MaxSH :type Float%20%28double-precision%29))
  (Default|UpdateSH (Variables|Default|GetHudWidget) CurSH MaxSH))

(fn BindPlayerState
  (params (PlayerState :type BP%20Shooting%20Player%20State%20Object%20Reference))
  (Development|PrintString "BindPlayerState" true true "(R=0.000000,G=0.660000,B=1.000000,A=1.000000)" 6e+01)
  (EventDispatchers|BindEventtoEventDispatcherChangeUserName PlayerState (EventDispatchers|CreateEvent :!event EventChangeUserName))
  (CallFunction|EventChangeUserName (Variables|/Game/Shooting/GameMode/InGame/BP_ShootingPlayerState.BP_ShootingPlayerState_C|GetUserName PlayerState))
  (EventDispatchers|BindEventtoEventDispatcherUpdateKillDeath PlayerState (EventDispatchers|CreateEvent :!event EventUpdateKillDeath))
  (CallFunction|EventUpdateKillDeath (Variables|/Game/Shooting/GameMode/InGame/BP_ShootingPlayerState.BP_ShootingPlayerState_C|GetKill PlayerState) (Variables|/Game/Shooting/GameMode/InGame/BP_ShootingPlayerState.BP_ShootingPlayerState_C|GetDeath PlayerState)))

(fn EventChangeUserName
  (params (UserName :type String))
  (bind _hudwidget (Variables|Default|GetHudWidget))
  (Development|PrintString (Utilities|String|Append "Event Change User Name - " UserName) true true "(R=0.000000,G=0.660000,B=1.000000,A=1.000000)" 6e+01)
  (Utilities|IsValid _hudwidget
    (:Is%20Valid
      (Default|UpdatePlayerList _hudwidget))))

(fn EventUpdateKillDeath
  (params (Kill :type Integer) (Death :type Integer))
  (bind _hudwidget (Variables|Default|GetHudWidget))
  (Development|PrintString (Utilities|String|Append "Event Update Kill : " (Utilities|String|ToString(Integer) Kill) ", Death : " (Utilities|String|ToString(Integer) Death)))
  (Utilities|IsValid _hudwidget
    (:Is%20Valid
      (Default|UpdatePlayerList _hudwidget))))