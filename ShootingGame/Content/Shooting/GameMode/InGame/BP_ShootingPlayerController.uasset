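; BP_ShootingPlayerController is the shooting game's player controller that passes each player's locally stored user name to their player state.
; On possession, the server calls a client event, which reads the name from BP_ShootingGameInstance and sends it back through a server request.
; The server then applies it with ChangeUserName on BP_ShootingPlayerState, completing a server-client-server round trip.
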(event Custom|EventOnPossessClient
  (params (PossessedPawn :type Pawn%20Object%20Reference))
  ;[1 1 1] (Client)
  (Development|PrintString "EventOnPossessClient" false false "(R=0.000000,G=0.660000,B=1.000000,A=1.000000)" 6e+01)
  (bind _asbp_shooting_game_instance (Utilities|Casting|CastToBP_ShootingGameInstance (Game|GetGameInstance)))
  (CallFunction|ReqNewUserName (Variables|/Game/Shooting/GameMode/BP_ShootingGameInstance.BP_ShootingGameInstance_C|GetUserName _asbp_shooting_game_instance)))

(event Custom|ReqNewUserName
  (params (NewUserName :type String))
  ;[1 0 0] (Server)
  (bind _asbp_shooting_player_state (Utilities|Casting|CastToBP_ShootingPlayerState (Variables|GetPlayerState)))
  (Default|ChangeUserName _asbp_shooting_player_state NewUserName))

(event EventPossess
  (params (PossessedPawn :type Pawn%20Object%20Reference))
  ;[1 0 0] (Server)
  (Development|PrintString (Utilities|String|Append "Event On Possess : " (Utilities|GetDisplayName PossessedPawn)) false false "(R=0.000000,G=0.660000,B=1.000000,A=1.000000)" 6e+01)
  (CallFunction|EventonPossessClient PossessedPawn))

(fn ConstructionScript)