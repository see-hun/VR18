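; Step actor for a VR step sequence that completes when the player selects it with a line trace.
; On step start it turns on the VRStepPawn's select line trace and enables its box collision, which is off at BeginPlay.
; Begin and end overlap toggle a decal highlight.
; A line-trace click disables trace, collision and decal, then ends the step.
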(event EventBeginPlay
  (|CallParentFunction)
  (Rendering|SetVisibility (Variables|Default|GetDecal) false false)
  (Collision|SetCollisionEnabled (Variables|Default|GetBox) "NoCollision"))

(fn ConstructionScript
  (|CallParentFunction))

(fn OnBeginOverlap
  (Rendering|SetVisibility (Variables|Default|GetDecal) true false))

(fn OnEndOverlap
  (Rendering|SetVisibility (Variables|Default|GetDecal) false false))

(fn EventStartStep
  (|CallParentFunction)
  (bind _asvrstep_pawn (Utilities|Casting|CastToVRStepPawn (Game|Player|GetPlayerPawn 0)))
  (Default|SetSelectLineTrace _asvrstep_pawn true)
  (Collision|SetCollisionEnabled (Variables|Default|GetBox) "QueryAndPhysics"))

(fn OnLineTraceClick
  (bind _asvrstep_pawn (Utilities|Casting|CastToVRStepPawn (Game|Player|GetPlayerPawn 0)))
  (Default|SetSelectLineTrace _asvrstep_pawn false)
  (Collision|SetCollisionEnabled (Variables|Default|GetBox) "NoCollision")
  (Rendering|SetVisibility (Variables|Default|GetDecal) false false)
  (CallFunction|EventEndStep))