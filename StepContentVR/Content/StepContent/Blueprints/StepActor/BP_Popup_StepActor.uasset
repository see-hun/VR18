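; Step actor that shows a popup widget with a title and description, optionally narrated, for the duration of its step.
; BeginPlay hides the widget, fills in its text and hooks the narration sound's finished event.
; Starting the step reveals the popup and plays the narration, ending when audio finishes or after a fixed timer if none is set.
; InitStep resets it by hiding the popup, stopping audio and clearing that timer.
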(event EventBeginPlay
  (|CallParentFunction)
  (Rendering|SetVisibility (Variables|Default|GetWidget) false false)
  (bind _aspopup_widget (Utilities|Casting|CastToPopupWidget (UserInterface|GetUserWidgetObject (Variables|Default|GetWidget))))
  (Default|SetPopupText _aspopup_widget (Variables|Default|GetTitle) (Variables|Default|GetDesc))
  (Audio|Components|Audio|SetSound (Variables|Default|GetAudio) (Variables|Default|GetNarr))
  (EventDispatchers|BindEventtoOnAudioFinished (Variables|Default|GetAudio) (EventDispatchers|CreateEvent :!event EventSoundFinish)))

(fn ConstructionScript
  (|CallParentFunction))

(fn EventStartStep
  (|CallParentFunction)
  (Rendering|SetVisibility (Variables|Default|GetWidget) true false)
  (Variables|Default|GetNarr
    (:then
      (Audio|Components|Audio|Play (Variables|Default|GetAudio) 0.0))
    (:else
      (Utilities|Time|SetTimerbyFunctionName 0 "EventEndStep" 5.0))))

(fn EventEndStep
  (|CallParentFunction)
  (Rendering|SetVisibility (Variables|Default|GetWidget) false false))

(fn EventSoundFinish
  (CallFunction|EventEndStep))

(fn InitStep
  (|CallParentFunction)
  (Utilities|FlowControl|Sequence
    (:then_0
      (Rendering|SetVisibility (Variables|Default|GetWidget) false false)
      (Audio|Components|Audio|Stop (Variables|Default|GetAudio)))
    (:then_1
      (if (Class|KismetSystemLibrary|TimerExists 0 "EventEndStep")
        (Utilities|Time|ClearTimerbyFunctionName 0 "EventEndStep")))))