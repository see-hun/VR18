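; Step actor that teleports the player pawn to a tagged PlayerStart as one step in the game's step system.
; Starting the step locks changes on BP_StepGameState and fades the camera out over five seconds.
; A timer then moves and rotates the pawn to the PlayerStart matching PlayerStartTag and fades back in.
; A second timer ends the step, re-enabling changes before calling the parent end logic.
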(fn ConstructionScript
  (|CallParentFunction))

(fn EventStartStep
  (|CallParentFunction)
  (bind _asbp_step_game_state (Utilities|Casting|CastToBP_StepGameState (Game|GetGameState)))
  (Default|SetCanChange _asbp_step_game_state false)
  (CameraFades|StartCameraFade :self (Game|GetPlayerCameraManager 0) :ToAlpha 1.0 :Duration 5.0 :bHoldWhenFinished true)
  (Utilities|Time|SetTimerbyFunctionName 0 "DoTeleport" 5.0))

(fn DoTeleport
  (bind _returnvalue (Game|GetGameMode))
  (bind _playerstarttag (Variables|Default|GetPlayerStartTag))
  (bind _returnvalue_2 (Class|GameModeBase|FindPlayerStart _returnvalue 0 _playerstarttag))
  (Transformation|SetActorLocationAndRotation (Game|Player|GetPlayerPawn 0) (Transformation|GetActorLocation _returnvalue_2) (Transformation|GetActorRotation _returnvalue_2))
  (CameraFades|StartCameraFade :self (Game|GetPlayerCameraManager 0) :FromAlpha 1.0 :Duration 5.0 :bHoldWhenFinished true)
  (Utilities|Time|SetTimerbyFunctionName 0 "EventEndStep" 5.0))

(fn EventEndStep
  (bind _asbp_step_game_state (Utilities|Casting|CastToBP_StepGameState (Game|GetGameState)))
  (Default|SetCanChange _asbp_step_game_state true)
  (|CallParentFunction))