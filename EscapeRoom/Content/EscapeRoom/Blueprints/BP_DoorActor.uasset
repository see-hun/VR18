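; Escape room door actor that swings open once every gimmick in its Gimmicks array is complete.
; On BeginPlay it binds to each gimmick's completion dispatcher, and the completion handler rechecks all gimmicks before opening.
; A Timeline drives the door mesh's yaw through a 90-degree swing.
; A close event reverses the Timeline, though nothing in this Blueprint calls it.
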(event Custom|DoCloseDoor
  (bind _rotationz (Timeline|Timeline ReverseFromEnd)
    (:Update
      (Transformation|SetRelativeRotation (Variables|Default|GetSM_Door) (Math|Rotator|MakeRotator 0.0 0.0 (* _rotationz -9e+01)) false false))))

(event Custom|DoOpenDoor
  (bind _rotationz (Timeline|Timeline PlayFromStart)
    (:Update
      (Transformation|SetRelativeRotation (Variables|Default|GetSM_Door) (Math|Rotator|MakeRotator 0.0 0.0 (* _rotationz -9e+01)) false false))))

(event EventBeginPlay
  (for _array_element (Variables|Default|GetGimmicks)
    (EventDispatchers|BindEventtoEventDispatcherComplate _array_element (EventDispatchers|CreateEvent :!event EventGimmickComplate))))

(fn ConstructionScript)

(fn EventGimmickComplate
  (params (IsComplate :type Boolean))
  (bind _isallcomplate (CallFunction|IsAllGimmickComplate))
  (if _isallcomplate
    (CallFunction|DoOpenDoor)))

(fn IsAllGimmickComplate
  (for _array_element (Variables|Default|GetGimmicks)
    (if (not (Variables|/Game/EscapeRoom/Blueprints/BP_Gimmick.BP_Gimmick_C|GetIsComplate _array_element))
      (return false)))
  (return true))