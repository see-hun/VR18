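; BP_Gimmick is an escape room gimmick that completes when checked against an item of the required type.
; On BeginPlay it looks up its RowName in DT_ItemTable and caches that row as MatchItem.
; OnCheckQuest compares item types and, on a match, removes MatchItem from the player pawn's BP_InvenComponent.
; It then runs EventQuestComplate to set the completion flag and fires the Complate dispatcher.
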(event EventBeginPlay
  (bind _returnvalue (Utilities|GetDataTableRow "/Game/EscapeRoom/Data/DT_ItemTable.DT_ItemTable" (Variables|Default|GetRowName))
    (:then
      (Variables|Default|SetMatchItem _returnvalue))))

(fn ConstructionScript)

(fn OnCheckQuest
  (params (Item :type ST%20Item%20Structure))
  (bind _output_get (Variables|Default|SetIsComplate (Utilities|Enum|Equal(Enum) (.ItemType (Utilities|Struct|BreakST_Item Item)) (.itemtype (Variables|Default|GetMatchItem)))))
  (if _output_get
    (Default|RemoveItem (Actor|GetComponentbyClass (Game|Player|GetPlayerPawn 0) "/Game/EscapeRoom/Blueprints/BP_InvenComponent.BP_InvenComponent_C") (Variables|Default|GetMatchItem))
    (CallFunction|EventQuestComplate)
    (Default|CallEventDispatcherComplate (Variables|Default|GetIsComplate))))

(fn EventQuestComplate
  (Variables|Default|SetIsComplate true))